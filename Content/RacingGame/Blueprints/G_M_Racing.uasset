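; Racing game mode that runs a timed race, won at the finish line or lost when time runs out.
; On BeginPlay it binds to the crossing event of finish-line Checkpoint actors, then runs a delayed start countdown.
; GameStart sets a timer for the out-of-time loss, which the win event clears.
; Both outcomes feed GameEnd, and race states and results appear only as printed strings.
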(event Custom|GameStart
  (Development|PrintString "Game Started")
  (bind _returnvalue (Utilities|Time|SetTimerbyEvent (delegate Custom|LoseOutOfTime) (Variables|Default|GetStart%20Timer%20Duration)))
  (Variables|Default|SetTime_RemainingTimer _returnvalue))

(event Custom|GameEnd
  (params (PlayerWon :type Boolean))
  (Development|PrintString (Utilities|String|SelectString "You Won" "You Lose" PlayerWon)))

(event Custom|Start%20Countdown
  (Development|PrintString "starting countdown")
  (Utilities|FlowControl|Delay (Variables|Default|GetStart%20Countdown%20Duration))
  (CallFunction|GameStart))

(event Custom|LoseOutOfTime
  (CallFunction|GameEnd false))

(event Custom|Win_CrossTheFinishLine
  (Utilities|Time|ClearandInvalidateTimerbyHandle (Variables|Default|GetTime_RemainingTimer))
  (CallFunction|GameEnd true))

(event EventBeginPlay
  (Utilities|FlowControl|Sequence
    (:then_0
      (bind _outactors (Actor|GetAllActorsOfClass "/Game/RacingGame/CheckPoints/Checkpoint.Checkpoint_C"))
      (for _array_element _outactors
        (if (Variables|/Game/RacingGame/CheckPoints/Checkpoint.Checkpoint_C|GetIsFinishLine _array_element)
          (EventDispatchers|BindEventtoOnCheckpoinCross _array_element (EventDispatchers|CreateEvent :!event Custom|Win_CrossTheFinishLine)))))
    (:then_1
      (CallFunction|StartCountdown))))

(event EventTick
  (params (DeltaSeconds :type Float%20%28single-precision%29)))

(fn ConstructionScript)